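; BP_FollowPlayerCamera is a platformer camera that smoothly follows BP_AG_1DPlayer along the world X axis.
; BeginPlay starts a fast looping timer that calls FollowPlayer, leaving Tick unused.
; Each call looks up the player by class and lerps the actor a small fraction toward the player's X, keeping its own Y and Z for an eased, lagging follow.
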(event EventBeginPlay
  (Utilities|Time|SetTimerbyFunctionName 0 "FollowPlayer" 0.01 true))

(event EventTick
  (params (DeltaSeconds :type Float%20%28single-precision%29)))

(fn ConstructionScript)

(fn FollowPlayer
  (bind _returnvalue (Transformation|GetActorLocation))
  ;[0.2061 1 0.3129] Camera Following Player In a Soothing Fashion
  (bind _returnvalue_2 (Actor|GetActorOfClass "/Game/Platformer/Blueprints/BP_AG_1DPlayer.BP_AG_1DPlayer_C"))
  (LocalVariables|SetPlayerLocation (Transformation|GetActorLocation _returnvalue_2))
  (Transformation|SetActorLocation (Math|Vector|Lerp(Vector) _returnvalue (+ _returnvalue (Math|Vector|MakeVector (- (.x (LocalVariables|GetPlayerLocation)) (.x (Transformation|GetActorLocation))) 0.0 0.0)) 0.01) false false))