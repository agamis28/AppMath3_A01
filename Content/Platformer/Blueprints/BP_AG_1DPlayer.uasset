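; Player Blueprint for a one-input, 1D platformer prototype in which a cube jumps vertically.
; BeginPlay adds the IMC_AG_1D Enhanced Input mapping context to the first player controller.
; Each Triggered movement event offsets the cube upward in world Z by JumpForce without sweep, shows the jump arrow and prints a debug message.
; The Completed event hides the arrow again.
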(event Input|EnhancedActionEvents|EnhancedInputActionIA_AG_1D_Movement
  (params (ActionValue :type Boolean) (ElapsedSeconds :type Float%20%28double-precision%29) (TriggeredSeconds :type Float%20%28double-precision%29) (InputAction :type Input%20Action%20Object%20Reference :default "/Game/Platformer/Core/Input/IA_AG_1D_Movement.IA_AG_1D_Movement"))
  (:Triggered
    (Transformation|SetWorldLocation (Variables|Default|GetCube) (+ (Transformation|GetWorldLocation (Variables|Default|GetCube)) (Math|Vector|MakeVector 0.0 0.0 (Variables|Default|GetJumpForce))) false false)
    (Development|SetHiddeninGame (Variables|Default|GetJumpArrow) false false)
    (Development|PrintString "Jumped"))
  (:Completed
    (Development|SetHiddeninGame (Variables|Default|GetJumpArrow) true false)))

(event EventBeginPlay
  ;[0 1 0.1458] BeginPlay
  ;[0 1 0.1458] Creating Mapping Context
  (Variables|Default|SetPlayerController (Game|GetPlayerController 0))
  (Input|AddMappingContext (PlayerController|LocalPlayerSubsystems|GetEnhancedInputLocalPlayerSubsystem (Variables|Default|GetPlayerController)) "/Game/Platformer/Core/Input/IMC_AG_1D.IMC_AG_1D" 0 "(bIgnoreAllPressedKeysUntilRelease=True,bForceImmediately=False,bNotifyUserSettings=False)"))

(fn ConstructionScript)